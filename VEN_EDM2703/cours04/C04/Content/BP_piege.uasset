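; BP_piege is a trap actor that drops a BP_Bloc when the first-person character steps into its box trigger.
; On overlap, it spawns the block 1000 units above itself with a limited lifespan and turns the cylinder red through a dynamic M_Pastille material created at BeginPlay.
; Nothing resets the color or limits retriggering, so each new player overlap spawns another block.
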(event `self.ReceiveBeginPlay`
  (bind _returnvalue (`PrimitiveComponent.CreateDynamicMaterialInstance` (`self.Cylinder`) 0 "/Game/M_Pastille.M_Pastille" "None"))
  (set `self.DynamicMat` _returnvalue))

(event `self.Box.OnComponentBeginOverlap`
  (params (OverlappedComponent :type "PrimitiveComponent Object Reference") (OtherActor :type "Actor Object Reference") (OtherComp :type "PrimitiveComponent Object Reference") (OtherBodyIndex :type Integer) (bFromSweep :type Boolean) (SweepResult :type "HitResult Structure (by ref)"))
  (cast `/Game/FirstPerson/Blueprints/BP_FirstPersonCharacter` OtherActor)
  (`|ExecutionSequence`
    (:`then_0`
      (bind _returnvalue (`|SpawnActorFromClass` "/Game/BP_Bloc.BP_Bloc_C" (`KismetMathLibrary.MakeTransform` (+ (`self.K2_GetActorLocation`) (0.0 0.0 1000.0))) "Undefined" "MultiplyWithRoot" null null))
      (`self.SetLifeSpan` _returnvalue 8.0))
    (:`then_1`
      (`MaterialInstanceDynamic.SetVectorParameterValue` (`self.DynamicMat`) "Color" (struct :`R` 1.0 :`A` 1.0)))))

(fn `UserConstructionScript`)