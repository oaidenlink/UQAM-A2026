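; BP_kum is an actor with a point light that moves and changes color on player key presses.
; It enables input for the first player controller on BeginPlay; X plays the Pos_lum timeline and Z reverses it.
; The timeline's scaled curves set the light's relative X/Y position, while its color track sets the light color.
; The Box overlap only casts to BP_FirstPersonCharacter and triggers nothing further.
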(event `self.Box.OnComponentBeginOverlap`
  (params (OverlappedComponent :type "PrimitiveComponent Object Reference") (OtherActor :type "Actor Object Reference") (OtherComp :type "PrimitiveComponent Object Reference") (OtherBodyIndex :type Integer) (bFromSweep :type Boolean) (SweepResult :type "HitResult Structure (by ref)"))
  (cast `/Game/FirstPerson/Blueprints/BP_FirstPersonCharacter` OtherActor))

(event `self.ReceiveBeginPlay`
  (`self.EnableInput` (`GameplayStatics.GetPlayerController` 0)))

(event `Key|X`
  (params (Key :type "Key Structure"))
  (bind _pointlight (`self.PointLight`))
  (:`Pressed`
    (bind (_direction _pos_x _pos_y _shapes_and_colors) (`Timeline|pos_lum` :!label _label)
      (:`Update`
        (`SceneComponent.K2_SetRelativeLocation` _pointlight (`KismetMathLibrary.MakeVector` (* _pos_x 1000.0) (* _pos_y 1000.0)) false false)
        (`LightComponent.SetLightColor` _pointlight _shapes_and_colors true)))))

(event `Key|Z`
  (params (Key :type "Key Structure"))
  (:`Pressed`
    (goto _label :!via `Reverse`)))

(fn `UserConstructionScript`)