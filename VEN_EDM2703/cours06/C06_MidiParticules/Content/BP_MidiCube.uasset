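; Actor that moves its Cube component vertically in response to MIDI control values.
; Tick maps the MIDI Value from the 0–127 range to a height and eases SmoothedValue toward it with FInterpTo, then sets the cube's relative Z.
; MIDIControl checks channel and controller ID before triggering the same location update, but the Tick-driven smoothing and movement bypass that filter.
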(event `/Game/BPI_MIDIInterface.MIDIControl`
  (params (Channel :type Integer) (ID :type Integer) (Value :type Integer))
  (if (== Channel (`self.MIDIChannel`))
    (if (== ID (`self.ID`))
      (`SceneComponent.K2_SetRelativeLocation` (`self.Cube`) (`KismetMathLibrary.MakeVector` 0.0 0.0 (stale `self.ReceiveTick` _output_get)) false false :!label _label))))

(event `self.ReceiveTick`
  (params (DeltaSeconds :type "Float (single-precision)"))
  (bind _output_get (set `self.SmoothedValue` (`KismetMathLibrary.FInterpTo` (`self.SmoothedValue`) (`KismetMathLibrary.MapRangeClamped` (`KismetMathLibrary.Conv_IntToDouble` (stale `/Game/BPI_MIDIInterface.MIDIControl` Value)) 0.0 127.0 0.0 1000.0) DeltaSeconds 0.9)))
  (goto _label))

(fn `UserConstructionScript`)