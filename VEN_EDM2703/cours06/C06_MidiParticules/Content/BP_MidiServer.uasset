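; BP_MidiServer is an actor that relays input from a MIDI device to interface-implementing actors in the level.
; On BeginPlay it opens a controller on a hardcoded device ID and caches all actors implementing BPI_MIDIInterface.
; Note On and Note Off events share one note message, while Control Change gets its own, each passing channel, ID and velocity.
; Device-listing and event-printing debug nodes are left unconnected.
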(event `self.ReceiveBeginPlay`
  (bind _returnvalue (`MIDIDeviceManager.CreateMIDIDeviceController` 1))
  (bind _output_get (set `self.MidiController` _returnvalue))
  (add `MIDIDeviceController.OnMIDIEvent` _output_get (delegate `MIDImsg`))
  (bind _outactors (`GameplayStatics.GetAllActorsWithInterface` "/Game/BPI_MIDIInterface.BPI_MIDIInterface_C"))
  (set `self.MidiInterfaced Actor` _outactors))

(event `MIDImsg`
  (params (MIDIDeviceController :type "MIDIDeviceController Object Reference") (Timestamp :type Integer) (EventType :type "EMIDIEventType Enum" :default "Unknown") (Channel :type Integer) (ControlID :type Integer) (Velocity :type Integer) (RawEventType :type Integer))
  (set `self.Channel` Channel)
  (set `self.Control ID` ControlID)
  (set `self.Velocity` Velocity)
  (switch `EMIDIEventType` EventType
    (:`NoteOff`
      (message `/Game/BPI_MIDIInterface.MIDINote` (`self.MidiInterfaced Actor`) (`self.Channel`) (`self.Control ID`) (`self.Velocity`) :!label _label))
    (:`NoteOn`
      (goto _label))
    (:`ControlChange`
      (message `/Game/BPI_MIDIInterface.MIDIControl` (`self.MidiInterfaced Actor`) (`self.Channel`) (`self.Control ID`) (`self.Velocity`)))))

(fn `UserConstructionScript`)